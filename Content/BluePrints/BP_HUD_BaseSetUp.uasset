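; BP_HUD_BaseSetUp is a HUD Blueprint that sets up the player's base on-screen interface.
; On BeginPlay it switches input to game-only, then creates, stores and displays the core HUD and character actions widgets for the owning player.
; Inventory and quests widget creation is present but disconnected, with a note that those menus will be controlled from the Player Controller.
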(event EventBeginPlay
  (Input|SetInputModeGameOnly (Game|Player|GetOwningPlayerController) false)
  ;[1 1 1 1 12] Game: Health, Emo account etc (((DESDE GAME MODE)))
  (bind _returnvalue (UserInterface|CreateWidget "/Game/BluePrints/WB_CoreWidget_HUD.WB_CoreWidget_HUD_C" (Game|Player|GetOwningPlayerController)))
  (bind _output_get (Variables|Default|SetWB_Core _returnvalue))
  (UserInterface|Viewport|AddtoViewport _output_get 0)
  (bind _returnvalue_2 (UserInterface|CreateWidget "/Game/Widgets/WB_CharacterActions.WB_CharacterActions_C" (Game|Player|GetOwningPlayerController)))
  (bind _output_get_2 (Variables|Default|SetWB_CharacterActions _returnvalue_2))
  (UserInterface|Viewport|AddtoViewport _output_get_2 0))

(fn ConstructionScript)